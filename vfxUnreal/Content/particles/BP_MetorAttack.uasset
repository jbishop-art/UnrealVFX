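; Meteor attack actor that plays an area-of-effect meteor shower effect when P is pressed, with input enabled on BeginPlay.
; P spawns a short-lived AOE ring decal at a fixed location, then after a delay activates the large and small meteor particle systems.
; Particle collision events spawn a matching explosion and temporary impact decal at each hit, sized by meteor type.
; The graph contains only visual effects, with no damage logic.
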(event OnParticleCollide(P_Meteor)
  (params (EventName :type Name :default "None") (EmitterTime :type Float%20%28single-precision%29) (ParticleTime :type Integer) (Location :type Vector :default "0, 0, 0") (Velocity :type Vector :default "0, 0, 0") (Direction :type Vector :default "0, 0, 0") (Normal :type Vector :default "0, 0, 0") (BoneName :type Name :default "None") (PhysMat :type Physical%20Material%20Object%20Reference))
  (Effects|SpawnEmitteratLocation "/Game/particles/P_Explosion_Big.P_Explosion_Big" Location "0, 0, 0" "5.000000,5.000000,5.000000")
  (Rendering|Decal|SpawnDecalatLocation "/Game/materials/M_Decal_Impact.M_Decal_Impact" "600.000000,600.000000,600.000000" Location "-90.000000,0.000000,-90.000000" 1.5))

(event OnParticleCollide(P_smallMeteors)
  (params (EventName :type Name :default "None") (EmitterTime :type Float%20%28single-precision%29) (ParticleTime :type Integer) (Location :type Vector :default "0, 0, 0") (Velocity :type Vector :default "0, 0, 0") (Direction :type Vector :default "0, 0, 0") (Normal :type Vector :default "0, 0, 0") (BoneName :type Name :default "None") (PhysMat :type Physical%20Material%20Object%20Reference))
  (Effects|SpawnEmitteratLocation "/Game/particles/P_Explosion_Small.P_Explosion_Small" Location)
  (Rendering|Decal|SpawnDecalatLocation "/Game/materials/M_Decal_Impact.M_Decal_Impact" "300.000000,300.000000,300.000000" Location "-90.000000,0.000000,90.000000" 1.5))

(event EventBeginPlay
  (Input|EnableInput 0))

(event Input|KeyboardEvents|P
  (params (Key :type Key%20Structure))
  (:Pressed
    (Rendering|Decal|SpawnDecalatLocation "/Game/materials/M_Decal_AOERing.M_Decal_AOERing" "1500.000000,1500.000000,1500.000000" "0.000000,500.000000, 0" "-90.000000,0.000000,-90.000000" 1.0)
    (Utilities|FlowControl|Delay 1.0)
    (Utilities|FlowControl|Sequence
      (:then_0
        (Components|Activation|Activate (Variables|Default|GetP_Meteor) true))
      (:then_1
        (Components|Activation|Activate (Variables|Default|GetP_smallMeteors) true)))))

(fn ConstructionScript)